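; VR movable drawer prototype that drives its static mesh by physics while held through a GrabComponent.
; On grab it stores the controller's offset from the mesh and opens a Tick gate, which closes on drop.
; While open, per-axis CalcAngle comparisons of current and starting offsets feed an acceleration-change torque on the mesh.
; A distance-scaled AddForce pull toward the hand is present but never runs.
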(event `self.ReceiveBeginPlay`)

(event `self.ReceiveTick`
  (params (DeltaSeconds :type "Float (single-precision)"))
  (`/Engine/EditorBlueprintResources/StandardMacros.Gate` true :!label _label
    (:`Exit`
      (`PrimitiveComponent.AddTorqueInDegrees` (`self.StaticMesh`) (`KismetMathLibrary.MakeVector` (`self.Calc_Angle` (`KismetMathLibrary.MakeVector` (.x (- (.location (`SceneComponent.K2_GetComponentToWorld` (`/Game/VRTemplate/Blueprints/GrabComponent.MotionControllerRef` (`self.GrabComponent`)))) (.location (`SceneComponent.K2_GetComponentToWorld` (`self.StaticMesh`)))))) (`KismetMathLibrary.MakeVector` (.x (.location (`self.Hand_Grab_Start_Relative`))))) (`self.Calc_Angle` (`KismetMathLibrary.MakeVector` 0.0 (.y (- (.location (`SceneComponent.K2_GetComponentToWorld` (`/Game/VRTemplate/Blueprints/GrabComponent.MotionControllerRef` (`self.GrabComponent`)))) (.location (`SceneComponent.K2_GetComponentToWorld` (`self.StaticMesh`)))))) (`KismetMathLibrary.MakeVector` 0.0 (.y (.location (`self.Hand_Grab_Start_Relative`))))) (`self.Calc_Angle` (`KismetMathLibrary.MakeVector` 0.0 0.0 (.z (- (.location (`SceneComponent.K2_GetComponentToWorld` (`/Game/VRTemplate/Blueprints/GrabComponent.MotionControllerRef` (`self.GrabComponent`)))) (.location (`SceneComponent.K2_GetComponentToWorld` (`self.StaticMesh`)))))) (`KismetMathLibrary.MakeVector` 0.0 0.0 (.z (.location (`self.Hand_Grab_Start_Relative`)))))) "None" true)
      (bind _output_get (set `self.cnt` (+ (`self.cnt`) 1)))
      (if (> _output_get 200)
        (set `self.cnt` 0)))))

(event `self.GrabComponent.OnGrabbed`
  (set `self.Hand_Grab_Start_Relative` (`KismetMathLibrary.MakeTransform` (- (.location (`SceneComponent.K2_GetComponentToWorld` (`/Game/VRTemplate/Blueprints/GrabComponent.MotionControllerRef` (`self.GrabComponent`)))) (.location (`SceneComponent.K2_GetComponentToWorld` (`self.StaticMesh`)))) (`KismetMathLibrary.NormalizedDeltaRotator` (.rotation (`SceneComponent.K2_GetComponentToWorld` (`/Game/VRTemplate/Blueprints/GrabComponent.MotionControllerRef` (`self.GrabComponent`)))) (.rotation (`SceneComponent.K2_GetComponentToWorld` (`self.StaticMesh`))))))
  (goto _label :!via `Open`))

(event `self.GrabComponent.OnDropped`
  (goto _label :!via `Close`))

(fn `UserConstructionScript`)