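; A configurable VR drawer that a motion controller grabs and slides along its Arrow's forward axis, with optional extension-based rotation about that axis.
; While grabbed, a gated Tick projects hand movement onto the axis, clamped by offset limits and max velocity.
; Looping movement audio scales pitch with extension and volume with speed; a DoOnce fires the end-stop sound at either limit.
; The construction script applies the mesh and placement offsets.
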(event `self.ReceiveBeginPlay`
  (set `self.Mesh_Start_Transform` (`SceneComponent.K2_GetComponentToWorld` (`self.MeshRoot`)))
  (set `self.Movement_Axis` (`SceneComponent.GetForwardVector` (`self.Arrow`)))
  (`KismetSystemLibrary.Delay` 0.2)
  (`PrimitiveComponent.SetCollisionResponseToChannel` (`self.StaticMesh`) "ECC_GameTraceChannel2" "ECR_Block"))

(event `self.ReceiveTick`
  (params (DeltaSeconds :type "Float (single-precision)"))
  (bind _new_offset (`self.New_Offset`))
  (bind _returnvalue (< (`KismetMathLibrary.Abs` (- _new_offset (`self.Min_Offset`))) 1.0))
  (bind _returnvalue_2 (< (`KismetMathLibrary.Abs` (- (`self.Max_Offset`) _new_offset)) 1.0))
  (`/Engine/EditorBlueprintResources/StandardMacros.Gate` true :!label _label
    (:`Exit`
      (`|ExecutionSequence`
        (:`then_0`
          (bind _output_get (set `self.New_Offset` (`self.Calc_Mesh_New_Offset`)))
          (set `self.Drawer_Extenstion_Alpha` (`KismetMathLibrary.NormalizeToRange` _output_get (`self.Min_Offset`) (`self.Max_Offset`)))
          (`SceneComponent.K2_SetWorldLocation` (`self.MeshRoot`) (`self.Clac_Mesh_New_World_Location`) false false)
          (if (`self.Apply_Extension_Based_Rotation`)
            (`SceneComponent.K2_SetWorldRotation` (`self.MeshRoot`) (`self.Calc_Extension_Based_Rotation`) false false)))
        (:`then_1`
          ;[1 1 1] DrawerAudio Adjustemnts (Moving Drawer)
          (`AudioComponent.SetPitchMultiplier` (`self.DrawerAudio`) (`KismetMathLibrary.MapRangeClamped` (`self.Drawer_Extenstion_Alpha`) 0.0 1.0 (`self.Min_Drawer_Audio_Pitch`) (`self.Max_Drawer_Audio_Pitch`)))
          (`AudioComponent.AdjustVolume` (`self.DrawerAudio`) 0.2 (`self.Calc_Velocity_Based_Audio_Volume`) "Linear")
          (`|ExecutionSequence`
            (:`then_0`
              (if (or (and (> (`self.New_Offset`) (`self.Last_Offset`)) _returnvalue_2) (and _returnvalue (< (`self.New_Offset`) (`self.Last_Offset`))))
                ;[1 1 1] Adjust and Play DrawerEndAudio
                (`/Engine/EditorBlueprintResources/StandardMacros.DoOnce` true :!label _label_2
                  (:`Completed`
                    (`AudioComponent.SetVolumeMultiplier` (`self.DrawerEndAudio`) (`self.Calc_Velocity_Based_Audio_Volume`))
                    (`AudioComponent.SetPitchMultiplier` (`self.DrawerEndAudio`) (`KismetMathLibrary.MapRangeClamped` (`self.Drawer_Extenstion_Alpha`) 0.0 1.0 (`self.Min_Drawer_Audio_Pitch`) (`self.Max_Drawer_Audio_Pitch`)))
                    (`AudioComponent.Play` (`self.DrawerEndAudio`) 0.05)))))
            (:`then_1`
              (if (and (not _returnvalue_2) (not _returnvalue))
                (goto _label_2 :!via `Reset`)))))
        (:`then_2`
          (set `self.Last_Offset` (`self.New_Offset`)))))))

(event `self.GrabComponent.OnGrabbed`
  (`self.Init_Tracking`)
  (`ActorComponent.Activate` (`self.DrawerAudio`) false)
  (goto _label :!via `Open`))

(event `self.GrabComponent.OnDropped`
  (`AudioComponent.AdjustVolume` (`self.DrawerAudio`) 0.2 0.0 "Linear")
  (goto _label :!via `Close`))

(fn `Init_Tracking`
  (set `self.Mesh_Grab_Start_Location` (`SceneComponent.K2_GetComponentLocation` (`self.MeshRoot`)))
  (set `self.Hand_Grab_Start_Location` (`SceneComponent.K2_GetComponentLocation` (`/Game/VRTemplate/Blueprints/GrabComponent.MotionControllerRef` (`self.GrabComponent`)))))

(fn `UserConstructionScript`
  (`StaticMeshComponent.SetStaticMesh` (`self.StaticMesh`) (`self.Mesh`))
  (`SceneComponent.K2_AddRelativeLocation` (`self.StaticMesh`) (.location (`self.StaticMesh_Placement_Offset`)) false false)
  (`SceneComponent.K2_AddRelativeRotation` (`self.StaticMesh`) (.rotation (`self.StaticMesh_Placement_Offset`)) false false)
  (`SceneComponent.K2_AddRelativeLocation` (`self.GrabComponent`) (.location (`self.GrabComponent_Placement_Offset`)) false false)
  (`SceneComponent.K2_AddRelativeRotation` (`self.GrabComponent`) (.rotation (`self.GrabComponent_Placement_Offset`)) false false))