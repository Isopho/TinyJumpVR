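; VR grabbable mesh that rotates around an anchor on a selectable X, Y or Z axis.
; While grabbed, Tick projects motion-controller movement onto the rotation plane for a signed angle, then rotates and/or moves the mesh, optionally gated by location- or rotation-based limit checks.
; On release, optional physics takes over, with the constraint freeing only that axis unless in manual mode.
; Movement and impact sounds scale with angular speed.
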(event `self.ReceiveBeginPlay`
  ;[1 1 1] Save initial tramsform for boundry and rotation calculations
  (set `self.Mesh_Start_Transform` (`SceneComponent.K2_GetComponentToWorld` (`self.StaticMesh`)))
  (`PhysicsConstraintComponent.SetConstrainedComponents` (`self.PhysicsConstraint`) null "None" (`self.StaticMesh`) "None")
  (set `self.Rotation_Plane_Normal` (`KismetMathLibrary.GreaterGreater_VectorRotator` (select `/Game/MyContent/Blueprints/Enums/RotationAxis` (`self.Rotation_Axis`) :`NewEnumerator0` (1.0 0.0 0.0) :`NewEnumerator1` (0.0 1.0 0.0) :`NewEnumerator2` (0.0 0.0 1.0) :!type "Vector Structure") (`SceneComponent.K2_GetComponentRotation` (`self.Root`))))
  (set `self.Initial_Orientation` (`SceneComponent.GetForwardVector` (`self.Arrow`)))
  (`KismetSystemLibrary.Delay` 0.2)
  (`PrimitiveComponent.SetCollisionResponseToChannel` (`self.StaticMesh`) "ECC_GameTraceChannel2" "ECR_Block"))

(event `self.ReceiveTick`
  (params (DeltaSeconds :type "Float (single-precision)"))
  (bind _movementaudio (`self.MovementAudio`))
  (bind _returnvalue (`SceneComponent.K2_GetComponentLocation` (`self.Anchor`)))
  (bind _returnvalue_2 (`KismetMathLibrary.RotatorFromAxisAndAngle` (`KismetMathLibrary.Normal` (`self.Rotation_Plane_Normal`)) (`self.Current_Rotation_Angle`)))
  (bind _returnvalue_3 (/ (`KismetMathLibrary.Abs` (- (`self.Last_Rotation_Angle`) (`self.Current_Rotation_Angle`))) (`GameplayStatics.GetWorldDeltaSeconds`)))
  (`/Engine/EditorBlueprintResources/StandardMacros.Gate` true :!label _label
    (:`Exit`
      (`|ExecutionSequence`
        (:`then_0`
          (`self.Calc_Current_Rotation_Angle`)
          (switch `/Game/MyContent/Blueprints/Enums/RotationCalculationMethod` (`self.Constraint_Calculation_Method`)
            (:`NewEnumerator2`
              (if (`self.Rotate_Mesh`) :!label _label_2
                (`SceneComponent.K2_SetWorldRotation` (`self.StaticMesh`) (`KismetMathLibrary.ComposeRotators` (.rotation (`self.Mesh_Grab_Start_Transform`)) _returnvalue_2) false false))
              (if (`self.Move_Mesh`)
                (`SceneComponent.K2_SetWorldLocation` (`self.StaticMesh`) (+ _returnvalue (`KismetMathLibrary.GreaterGreater_VectorRotator` (- (.location (`self.Mesh_Grab_Start_Transform`)) _returnvalue) _returnvalue_2)) true false))
              (`/Engine/EditorBlueprintResources/StandardMacros.DoOnce` false :!label _label_3
                (:`Completed`
                  (`KismetSystemLibrary.PrintString` (`KismetStringLibrary.Conv_DoubleToString` _returnvalue_3))
                  (`AudioComponent.Play` _movementaudio 0.0)
                  (`AudioComponent.SetVolumeMultiplier` _movementaudio (* (`KismetMathLibrary.RandomFloatInRange` 0.5 1.0) (`self.Base Audio Multiplyer`) (`KismetMathLibrary.FClamp` (/ _returnvalue_3 360.0))))
                  (`KismetSystemLibrary.Delay` (`KismetMathLibrary.RandomFloatInRange` 1.5 3.0))
                  (goto _label_3 :!via `Reset`))))
            (:`NewEnumerator0`
              (if (`self.Calc_Constrains_Based_On_Location`)
                (goto _label_2)))
            (:`NewEnumerator1`
              (if (`self.Calc_Constrains_Based_On_Rotation`)
                (goto _label_2)))))
        (:`then_1`
          (set `self.Last_Rotation_Angle` (`self.Current_Rotation_Angle`)))))))

(event `self.GrabComponent.OnGrabbed`
  (`PrimitiveComponent.SetSimulatePhysics` (`self.StaticMesh`) false)
  (`self.Init_Tracking`)
  (goto _label :!via `Open`))

(event `self.GrabComponent.OnDropped`
  (`PrimitiveComponent.SetSimulatePhysics` (`self.StaticMesh`) (`self.Simulate_Main_Mesh_Physics`))
  (goto _label :!via `Close`))

(event `self.StaticMesh.OnComponentHit`
  (params (HitComponent :type "PrimitiveComponent Object Reference") (OtherActor :type "Actor Object Reference") (OtherComp :type "PrimitiveComponent Object Reference") (NormalImpulse :type "Vector Structure") (Hit :type "HitResult Structure (by ref)"))
  (bind _hit_sound (`self.Hit Sound`))
  (if (< (`KismetArrayLibrary.Array_Find` (`self.No Sound Actors`) OtherActor) 0)
    (set `self.Hit Location` Hit_ImpactPoint)
    (`self.Calc_Hit_Volume` Hit_Normal (`self.StaticMesh`) OtherComp)
    (`/Engine/EditorBlueprintResources/StandardMacros.DoOnce` false :!label _label_4
      (:`Completed`
        (`GameplayStatics.PlaySoundAtLocation` _hit_sound (`self.Hit Location`) (struct) (`self.Hit Volume Multiplier`) 1.0 0.0 "/Game/Audio/_Mix/ATT_Emitter_SHRT.ATT_Emitter_SHRT" null null)
        (`KismetSystemLibrary.Delay` (* (`SoundBase.Duration` _hit_sound) 0.8))
        (goto _label_4 :!via `Reset`)))))

(fn `Calc_Current_Rotation_Angle`
  (bind _returnvalue (`KismetMathLibrary.Normal` (`self.Rotation_Plane_Normal`)))
  (bind _returnvalue_2 (`SceneComponent.K2_GetComponentLocation` (`self.Anchor`)))
  (bind _returnvalue_3 (`KismetMathLibrary.Normal` (`KismetMathLibrary.ProjectVectorOnToPlane` (- _returnvalue_2 (`self.Hand_Grab_Start_Location`)) _returnvalue)))
  (bind _returnvalue_4 (`KismetMathLibrary.Normal` (`KismetMathLibrary.ProjectVectorOnToPlane` (- _returnvalue_2 (`SceneComponent.K2_GetComponentLocation` (`/Game/VRTemplate/Blueprints/GrabComponent.MotionControllerRef` (`self.GrabComponent`)))) _returnvalue)))
  (set `self.Current_Rotation_Angle` (* (`KismetMathLibrary.DegAcos` (`KismetMathLibrary.Dot_VectorVector` _returnvalue_4 _returnvalue_3)) (`KismetMathLibrary.SelectFloat` 1.0 -1.0 (< (`KismetMathLibrary.Dot_VectorVector` (`KismetMathLibrary.Cross_VectorVector` _returnvalue_4 _returnvalue_3) (`KismetMathLibrary.Normal` (`self.Rotation_Plane_Normal`))) 0.0)))))

(fn `Calc_Hit_Volume`
  (params (Target :type "Vector Structure") (this :type "PrimitiveComponent Object Reference") (other :type "PrimitiveComponent Object Reference"))
  (set `self.Hit Volume Multiplier` (* (`KismetMathLibrary.FClamp` (/ (`KismetMathLibrary.VSize` (`PrimitiveComponent.GetPhysicsAngularVelocityInDegrees` this "None")) 360.0)) (`self.Base Audio Multiplyer`))))

(fn `Init_Tracking`
  (set `self.Mesh_Grab_Start_Transform` (`SceneComponent.K2_GetComponentToWorld` (`self.StaticMesh`)))
  (set `self.Hand_Grab_Start_Location` (`SceneComponent.K2_GetComponentLocation` (`/Game/VRTemplate/Blueprints/GrabComponent.MotionControllerRef` (`self.GrabComponent`))))
  (set `self.Grab_Start_Orientation` (`SceneComponent.GetForwardVector` (`self.Arrow`)))
  (set `self.Last_Rotation_Angle` 0.0)
  (set `self.Current_Rotation_Angle` 0.0))

(fn `UserConstructionScript`
  (`StaticMeshComponent.SetStaticMesh` (`self.StaticMesh`) (`self.Mesh`))
  (`SceneComponent.K2_AddRelativeLocation` (`self.StaticMesh`) (.location (`self.Static_Mesh_Placement_Offset`)) false false)
  (`SceneComponent.K2_AddRelativeRotation` (`self.StaticMesh`) (.rotation (`self.Static_Mesh_Placement_Offset`)) false false)
  (`SceneComponent.K2_AddRelativeLocation` (`self.GrabComponent`) (.location (`self.GrabComponent_Placement_Offset`)) false false)
  (`SceneComponent.K2_AddRelativeRotation` (`self.GrabComponent`) (.rotation (`self.GrabComponent_Placement_Offset`)) false false)
  (if (not (`self.PhysicsConstraint_Manual_Mode`))
    (`PhysicsConstraintComponent.SetAngularTwistLimit` (`self.PhysicsConstraint`) "ACM_Locked" 0.0)
    (`PhysicsConstraintComponent.SetAngularSwing2Limit` (`self.PhysicsConstraint`) "ACM_Locked" 0.0)
    (`PhysicsConstraintComponent.SetAngularSwing1Limit` (`self.PhysicsConstraint`) "ACM_Locked" 0.0)
    (switch `/Game/MyContent/Blueprints/Enums/RotationAxis` (`self.Rotation_Axis`)
      (:`NewEnumerator0`
        (`PhysicsConstraintComponent.SetAngularTwistLimit` (`self.PhysicsConstraint`) "ACM_Free" 0.0))
      (:`NewEnumerator1`
        (`PhysicsConstraintComponent.SetAngularSwing2Limit` (`self.PhysicsConstraint`) "ACM_Free" 0.0))
      (:`NewEnumerator2`
        (`PhysicsConstraintComponent.SetAngularSwing1Limit` (`self.PhysicsConstraint`) "ACM_Free" 0.0)))))