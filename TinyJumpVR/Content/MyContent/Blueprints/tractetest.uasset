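; Test actor that repeatedly fires a debug sphere trace from its Arrow component.
; From BeginPlay, a self-looping Delay repeats a short-range, small-radius trace along the arrow's forward vector on the TraceTypeQuery4 channel every few seconds, drawing it briefly.
; Branches check the return value and blocking hit, but both lead to no actions.
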(event `self.ReceiveBeginPlay`
  (bind _arrow (`self.Arrow`))
  (bind _returnvalue (`SceneComponent.K2_GetComponentLocation` _arrow))
  (bind (_outhit _returnvalue_2) (`KismetSystemLibrary.SphereTraceSingle` :`Start` _returnvalue :`End` (+ _returnvalue (* (`KismetMathLibrary.Normal` (`SceneComponent.GetForwardVector` _arrow)) (1000.0 1000.0 1000.0))) :`Radius` 6.0 :`TraceChannel` "TraceTypeQuery4" :`DrawDebugType` "ForDuration" :`DrawTime` 2.5 :!label _label))
  (if _returnvalue_2
    _
    (else
      _))
  (if (`GameplayStatics.BreakHitResult` _outhit)
    _
    (else
      _))
  (`KismetSystemLibrary.Delay` 3.0)
  (goto _label))

(fn `UserConstructionScript`)