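; VR grabbable physics mesh, such as a drawer, that slides along an arrow axis between min and max offsets.
; BeginPlay centers and sizes a physics constraint to that range.
; While grabbed, Tick projects controller movement onto the axis and applies distance-scaled force toward that target, cutting out nearby so damping smooths the stop.
; Velocity drives movement audio volume, while impact speed along the hit normal scales rate-limited hit sounds.
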(event `self.ReceiveBeginPlay`
  (bind _output_get (set `self.Mesh_Start_Transform` (`SceneComponent.K2_GetComponentToWorld` (`self.StaticMesh`))))
  ;[1 1 1] Adjust PhysicsConstraint to enforce the Min_Offset and Max_Offset
  (`SceneComponent.K2_SetWorldLocation` (`self.Anchor`) (+ (.location _output_get) (* (`KismetMathLibrary.Normal` (`SceneComponent.GetForwardVector` (`self.Arrow`))) (/ (+ (`self.Max_Offset`) (`self.Min_Offset`)) 2.0))) false false)
  (`SceneComponent.K2_SetWorldLocation` (`self.PhysicsConstraint`) (+ (.location _output_get) (* (`KismetMathLibrary.Normal` (`SceneComponent.GetForwardVector` (`self.Arrow`))) (/ (+ (`self.Max_Offset`) (`self.Min_Offset`)) 2.0))) false false)
  (`PhysicsConstraintComponent.SetLinearXLimit` (`self.PhysicsConstraint`) "LCM_Limited" (`KismetMathLibrary.Abs` (/ (- (`self.Max_Offset`) (`self.Min_Offset`)) 2.0)))
  (`KismetSystemLibrary.Delay` 0.2)
  (`PrimitiveComponent.SetCollisionResponseToChannel` (`self.StaticMesh`) "ECC_GameTraceChannel2" "ECR_Block")
  (`PrimitiveComponent.SetCollisionResponseToChannel` (`self.StaticMesh2`) "ECC_GameTraceChannel2" "ECR_Block"))

(event `self.ReceiveTick`
  (params (DeltaSeconds :type "Float (single-precision)"))
  (bind _returnvalue (+ (.location (`self.Mesh_Start_Transform`)) (* (`KismetMathLibrary.Normal` (`KismetMathLibrary.GetForwardVector` (`SceneComponent.K2_GetComponentRotation` (`self.Arrow`)))) (`self.New_Offset`))))
  (bind _returnvalue_2 (- (.location (`self.Mesh_Start_Transform`)) (+ (`self.Mesh_Grab_Start_Location`) (`KismetMathLibrary.ProjectVectorOnToVector` (- (`SceneComponent.K2_GetComponentLocation` (`/Game/VRTemplate/Blueprints/GrabComponent.MotionControllerRef` (`self.GrabComponent`))) (`self.Hand_Grab_Start_Location`)) (`KismetMathLibrary.GetForwardVector` (.rotation (`self.Mesh_Start_Transform`)))))))
  (bind _returnvalue_3 (`KismetMathLibrary.FClamp` (/ (`KismetMathLibrary.VSize` (- (`SceneComponent.K2_GetComponentLocation` (`self.StaticMesh`)) _returnvalue)) (`self.Max_Force_Distance`))))
  (`/Engine/EditorBlueprintResources/StandardMacros.Gate` true :!label _label
    (:`Exit`
      (`|ExecutionSequence`
        (:`then_0`
          (set `self.New_Offset` (`KismetMathLibrary.FClamp` (* (`KismetMathLibrary.VSize` _returnvalue_2) (`KismetMathLibrary.SelectFloat` 1.0 -1.0 (< (`KismetMathLibrary.Dot_VectorVector` _returnvalue_2 (`KismetMathLibrary.GetForwardVector` (.rotation (`self.Mesh_Start_Transform`)))) 0.0))) (`self.Min_Offset`) (`self.Max_Offset`)))
          ;[1 1 1] Disableing when close to target allows the Dampening to take over for a smooth transition
          (if (> _returnvalue_3 0.1)
            (`PrimitiveComponent.AddForce` (`self.StaticMesh`) (* (`KismetMathLibrary.GetDirectionUnitVector` (`SceneComponent.K2_GetComponentLocation` (`self.StaticMesh`)) _returnvalue) (`KismetMathLibrary.Lerp` 0.0 (`self.Drawing_Force`) _returnvalue_3)) "None" false)))
        (:`then_1`
          (bind _returnvalue_4 (`PrimitiveComponent.GetPhysicsLinearVelocity` (`self.StaticMesh`) "None"))
          (`AudioComponent.AdjustVolume` (`self.MovementAudio`) 0.2 (* (`KismetMathLibrary.FClamp` (/ (`KismetMathLibrary.VSize` _returnvalue_4) 100.0)) (`self.Base Audio Multiplyer`)) "Linear"))))))

(event `self.GrabComponent.OnGrabbed`
  (`self.Init_Tracking`)
  (`ActorComponent.Activate` (`self.MovementAudio`) false)
  (goto _label :!via `Open`))

(event `self.GrabComponent.OnDropped`
  (`AudioComponent.AdjustVolume` (`self.MovementAudio`) 0.2 0.0 "Linear")
  (goto _label :!via `Close`))

(event `self.StaticMesh.OnComponentHit`
  (params (HitComponent :type "PrimitiveComponent Object Reference") (OtherActor :type "Actor Object Reference") (OtherComp :type "PrimitiveComponent Object Reference") (NormalImpulse :type "Vector Structure") (Hit :type "HitResult Structure (by ref)"))
  (bind _hit_sound (`self.Hit Sound`))
  (set `self.Hit Location` Hit_ImpactPoint)
  (`self.Calc_Hit_Volume` Hit_Normal (`self.StaticMesh`) OtherComp)
  (if (> (`self.Hit Volume Multiplier`) 0.1)
    (`/Engine/EditorBlueprintResources/StandardMacros.DoOnce` false :!label _label_2
      (:`Completed`
        (`GameplayStatics.PlaySoundAtLocation` _hit_sound (`self.Hit Location`) (struct) (`self.Hit Volume Multiplier`) 1.0 0.0 "/Game/Audio/_Mix/ATT_Emitter_SHRT.ATT_Emitter_SHRT" null null)
        (`KismetSystemLibrary.Delay` (* (`SoundBase.Duration` _hit_sound) 0.8))
        (goto _label_2 :!via `Reset`)))))

(fn `Calc_Hit_Volume`
  (params (Target :type "Vector Structure") (this :type "PrimitiveComponent Object Reference") (other :type "PrimitiveComponent Object Reference"))
  (bind _returnvalue (`PrimitiveComponent.GetPhysicsLinearVelocity` this "None"))
  (bind _returnvalue_2 (`PrimitiveComponent.GetPhysicsLinearVelocity` other "None"))
  (set `self.Hit Volume Multiplier` (* (`KismetMathLibrary.FClamp` (/ (`KismetMathLibrary.VSize` (`KismetMathLibrary.ProjectVectorOnToVector` (- _returnvalue _returnvalue_2) Target)) 50.0)) (`self.Base Audio Multiplyer`))))

(fn `Init_Tracking`
  (set `self.Mesh_Grab_Start_Location` (`SceneComponent.K2_GetComponentLocation` (`self.StaticMesh`)))
  (set `self.Hand_Grab_Start_Location` (`SceneComponent.K2_GetComponentLocation` (`/Game/VRTemplate/Blueprints/GrabComponent.MotionControllerRef` (`self.GrabComponent`)))))

(fn `UserConstructionScript`)