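; BeamTest is a test Blueprint that sizes a Niagara menu beam using a forward line trace.
; Each tick it traces the Visibility channel from the root component out to InteractionDistance, drawing the debug line for one frame.
; The hit distance feeds the X of the User.BeamEnd vector on MenuBeamSystemRight, with no check for whether the trace hit.
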(event `self.ReceiveTick`
  (params (DeltaSeconds :type "Float (single-precision)"))
  (bind _returnvalue (`SceneComponent.K2_GetComponentLocation` (`self.DefaultSceneRoot`)))
  (bind _outhit (`KismetSystemLibrary.LineTraceSingle` :`Start` _returnvalue :`End` (+ _returnvalue (* (`SceneComponent.GetForwardVector` (`self.DefaultSceneRoot`)) (`self.InteractionDistance`))) :`TraceChannel` "TraceTypeQuery1" :`DrawDebugType` "ForOneFrame"))
  (`FXSystemComponent.SetVectorParameter` (`self.MenuBeamSystemRight`) "User.BeamEnd" (`KismetMathLibrary.MakeVector` (`.Distance` (`GameplayStatics.BreakHitResult` _outhit)))))

(fn `UserConstructionScript`)