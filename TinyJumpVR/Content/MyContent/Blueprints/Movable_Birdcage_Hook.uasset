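; Movable birdcage hook that a VR player grabs and slides along a single axis, the mesh's initial forward vector.
; Grabbing records mesh and hand start locations and opens a Tick gate; dropping closes it.
; While held, Tick projects the motion controller's movement onto that axis and sweeps the mesh there.
; Moves apply only while the signed distance from the BeginPlay position stays within the min and max offsets.
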(event `self.ReceiveBeginPlay`
  (set `self.Mesh_Start_Transform` (`SceneComponent.K2_GetComponentToWorld` (`self.StaticMesh`))))

(event `self.ReceiveTick`
  (params (DeltaSeconds :type "Float (single-precision)"))
  (bind _returnvalue (+ (`self.Mesh_Grab_Start_Location`) (`KismetMathLibrary.ProjectVectorOnToVector` (- (`SceneComponent.K2_GetComponentLocation` (`/Game/VRTemplate/Blueprints/GrabComponent.MotionControllerRef` (`self.GrabComponent`))) (`self.Hand_Grab_Start_Location`)) (`KismetMathLibrary.GetForwardVector` (.rotation (`self.Mesh_Start_Transform`))))))
  (bind _returnvalue_2 (- (.location (`self.Mesh_Start_Transform`)) _returnvalue))
  (bind _returnvalue_3 (* (`KismetMathLibrary.VSize` _returnvalue_2) (`KismetMathLibrary.SelectFloat` 1.0 -1.0 (< (`KismetMathLibrary.Dot_VectorVector` _returnvalue_2 (`KismetMathLibrary.GetForwardVector` (.rotation (`self.Mesh_Start_Transform`)))) 0.0))))
  (`/Engine/EditorBlueprintResources/StandardMacros.Gate` true :!label _label
    (:`Exit`
      (if (and (>= _returnvalue_3 (`self.Min_Offset`)) (<= _returnvalue_3 (`self.Max_Offset`)))
        (`SceneComponent.K2_SetWorldLocation` (`self.StaticMesh`) _returnvalue true false)))))

(event `self.GrabComponent.OnGrabbed`
  (`self.Init_Tracking`)
  (goto _label :!via `Open`))

(event `self.GrabComponent.OnDropped`
  (goto _label :!via `Close`))

(fn `Init_Tracking`
  (set `self.Mesh_Grab_Start_Location` (`SceneComponent.K2_GetComponentLocation` (`self.StaticMesh`)))
  (set `self.Hand_Grab_Start_Location` (`SceneComponent.K2_GetComponentLocation` (`/Game/VRTemplate/Blueprints/GrabComponent.MotionControllerRef` (`self.GrabComponent`)))))

(fn `UserConstructionScript`)