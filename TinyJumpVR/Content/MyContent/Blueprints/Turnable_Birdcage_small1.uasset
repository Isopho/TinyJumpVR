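; VR-grabbable birdcage mount that swings StaticMesh around an Anchor, with the Birdcage attached to it by a physics constraint.
; While grabbed, a gated Tick measures the hand's signed angle since grab start on the rotation plane.
; Within min/max offsets it sweeps the mesh's location along that arc; the rotation update is disconnected.
; A tiny force on the Birdcage after each move keeps the constraint from glitching.
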(event `self.ReceiveBeginPlay`
  ;[1 1 1] Save initial tramsform for boundry and rotation calculations
  (set `self.Mesh_Start_Transform` (`SceneComponent.K2_GetComponentToWorld` (`self.StaticMesh`)))
  (`PhysicsConstraintComponent.SetConstrainedComponents` (`self.PhysicsConstraint`) (`self.StaticMesh`) "None" (`self.Birdcage`) "None"))

(event `self.ReceiveTick`
  (params (DeltaSeconds :type "Float (single-precision)"))
  (bind _returnvalue (`KismetMathLibrary.Normal` (`self.Rotation_Plane_Normal`)))
  (bind _returnvalue_2 (`SceneComponent.K2_GetComponentLocation` (`self.Anchor`)))
  (bind _returnvalue_3 (`SceneComponent.K2_GetComponentLocation` (`self.Anchor`)))
  (bind _returnvalue_4 (`KismetMathLibrary.Normal` (`KismetMathLibrary.ProjectVectorOnToPlane` (- _returnvalue_2 (`self.Hand_Grab_Start_Location`)) _returnvalue)))
  (bind _returnvalue_5 (`KismetMathLibrary.Normal` (`KismetMathLibrary.ProjectVectorOnToPlane` (- _returnvalue_2 (`SceneComponent.K2_GetComponentLocation` (`/Game/VRTemplate/Blueprints/GrabComponent.MotionControllerRef` (`self.GrabComponent`)))) _returnvalue)))
  (bind _returnvalue_6 (* (`KismetMathLibrary.DegAcos` (`KismetMathLibrary.Dot_VectorVector` _returnvalue_5 _returnvalue_4)) (`KismetMathLibrary.SelectFloat` 1.0 -1.0 (< (`KismetMathLibrary.Dot_VectorVector` (`KismetMathLibrary.Cross_VectorVector` _returnvalue_5 _returnvalue_4) _returnvalue) 0.0))))
  (`/Engine/EditorBlueprintResources/StandardMacros.Gate` true :!label _label
    (:`Exit`
      (if (and (>= _returnvalue_6 (`self.Min_Offset_Degrees`)) (<= _returnvalue_6 (`self.Max_Offset_Degrees`)))
        (`SceneComponent.K2_SetWorldLocation` (`self.StaticMesh`) (+ _returnvalue_3 (`KismetMathLibrary.GreaterGreater_VectorRotator` (- (.location (`self.Mesh_Grab_Start_Transform`)) _returnvalue_3) (`KismetMathLibrary.MakeRotator` (* (.x _returnvalue) _returnvalue_6) (* (.y _returnvalue) _returnvalue_6) (* (.z _returnvalue) _returnvalue_6)))) true false)
        ;[1 1 1] needed so that the physicsContraint does not bug out
        (`PrimitiveComponent.AddForce` (`self.Birdcage`) (1.0 0.0 0.0) "None" false)
        (set `self.cnt` (+ (`self.cnt`) 1))
        (if (> (`self.cnt`) 50)
          (set `self.cnt` 0))))))

(event `self.GrabComponent.OnGrabbed`
  (`self.Init_Tracking`)
  (goto _label :!via `Open`))

(event `self.GrabComponent.OnDropped`
  (goto _label :!via `Close`))

(fn `Init_Tracking`
  (set `self.Mesh_Grab_Start_Transform` (`SceneComponent.K2_GetComponentToWorld` (`self.StaticMesh`)))
  (set `self.Hand_Grab_Start_Location` (`SceneComponent.K2_GetComponentLocation` (`/Game/VRTemplate/Blueprints/GrabComponent.MotionControllerRef` (`self.GrabComponent`)))))

(fn `UserConstructionScript`)