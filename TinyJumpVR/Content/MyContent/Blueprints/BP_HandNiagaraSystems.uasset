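; Hand particle effect with local-space and world-space Niagara systems that react to the closest grabbable object.
; An UpdateNiagaraSystem event, bound at BeginPlay, receives the grabbable and measures its distance from the root.
; Within detection range, both systems' color eases between two colors by distance, the world-space particles are attracted to the object, and a debug arrow is drawn.
; Otherwise, attraction strength turns slightly negative.
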(event `self.ReceiveBeginPlay`
  (`FXSystemComponent.SetColorParameter` (`self.NiagaraLS`) "User.ParticleColor" (`KismetMathLibrary.Conv_ColorToLinearColor` (`self.ParticleColor1`)))
  (`FXSystemComponent.SetColorParameter` (`self.NiagaraWS`) "User.ParticleColor" (`KismetMathLibrary.Conv_ColorToLinearColor` (`self.ParticleColor1`)))
  (add `self.UpdateNiagaraSystem` (delegate `UpdateNiagaraSystem_Event`)))

(event `UpdateNiagaraSystem_Event` :!signature `self.UpdateNiagaraSystem`
  (params (Grabable :type "SceneComponent Object Reference"))
  (bind _returnvalue (`SceneComponent.K2_GetComponentLocation` (`self.DefaultSceneRoot`)))
  (bind _returnvalue_2 (`SceneComponent.K2_GetComponentLocation` (`self.Closest_Grabable`)))
  (bind _output_get (set `self.Closest_Grabable` Grabable))
  (if (`KismetSystemLibrary.IsValid` _output_get)
    (bind _output_get_2 (set `self.Closest_Grabable_Distance` (`KismetMathLibrary.Abs` (`KismetMathLibrary.VSize` (- _returnvalue _returnvalue_2)))))
    (if (<= _output_get_2 (`self.DetectionRange`))
      (`KismetSystemLibrary.DrawDebugArrow` _returnvalue _returnvalue_2 1.0 (struct :`R` 1.0 :`B` 0.929991 :`A` 1.0) 0.1 0.5)
      (`FXSystemComponent.SetColorParameter` (`self.NiagaraWS`) "User.ParticleColor" (`KismetMathLibrary.LinearColorLerp` (`KismetMathLibrary.Conv_ColorToLinearColor` (`self.ParicalColor2`)) (`KismetMathLibrary.Conv_ColorToLinearColor` (`self.ParticleColor1`)) (`|EaseFunction` "EaseInOut" (`KismetMathLibrary.FClamp` (/ (`self.Closest_Grabable_Distance`) (`self.DetectionRange`))) 0.0 1.0)))
      (`FXSystemComponent.SetColorParameter` (`self.NiagaraLS`) "User.ParticleColor" (`KismetMathLibrary.LinearColorLerp` (`KismetMathLibrary.Conv_ColorToLinearColor` (`self.ParicalColor2`)) (`KismetMathLibrary.Conv_ColorToLinearColor` (`self.ParticleColor1`)) (`|EaseFunction` "EaseInOut" (`KismetMathLibrary.FClamp` (/ (`self.Closest_Grabable_Distance`) (`self.DetectionRange`))) 0.0 1.0)))
      (`FXSystemComponent.SetVectorParameter` (`self.NiagaraWS`) "User.AttractionPoint" (`SceneComponent.K2_GetComponentLocation` (`self.Closest_Grabable`)))
      (`FXSystemComponent.SetFloatParameter` (`self.NiagaraWS`) "User.AttractionStrength" 2.0)
      (else
        (`FXSystemComponent.SetFloatParameter` (`self.NiagaraWS`) "User.AttractionStrength" -0.1 :!label _label)))
    (else
      (goto _label))))

(fn `UserConstructionScript`)