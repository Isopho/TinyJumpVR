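; VR spring-loaded drawable object that a motion controller can grab and slide along a single axis.
; While it is grabbed, a gate lets Tick move HandAnchor with the controller at the offset captured on grab; dropping snaps the anchor back to the mesh.
; Each Tick projects the physics mesh onto the Arrow axis through LocationAnchor, clamps its offset to MinOff/MaxOff and applies a tiny force.
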(event `self.ReceiveBeginPlay`)

(event `self.ReceiveTick`
  (params (DeltaSeconds :type "Float (single-precision)"))
  (bind _returnvalue (`SceneComponent.K2_GetComponentLocation` (`self.MovableStaticMesh`)))
  (bind _returnvalue_2 (`KismetMathLibrary.Normal` (`SceneComponent.GetForwardVector` (`self.Arrow`))))
  (bind _returnvalue_3 (- (`SceneComponent.K2_GetComponentLocation` (`self.LocationAnchor`)) _returnvalue))
  (bind _returnvalue_4 (`KismetMathLibrary.VSize` (`KismetMathLibrary.ProjectVectorOnToVector` _returnvalue_3 _returnvalue_2)))
  (`|ExecutionSequence`
    (:`then_0`
      (`/Engine/EditorBlueprintResources/StandardMacros.Gate` true :!label _label
        (:`Exit`
          (`SceneComponent.K2_SetWorldLocation` (`self.HandAnchor`) (+ (`SceneComponent.K2_GetComponentLocation` (`/Game/VRTemplate/Blueprints/GrabComponent.MotionControllerRef` (`self.GrabComponent`))) (`self.deifVec`)) false false))))
    (:`then_1`
      (`SceneComponent.K2_SetWorldLocation` (`self.MovableStaticMesh`) (+ (+ _returnvalue (`KismetMathLibrary.ProjectVectorOnToPlane` _returnvalue_3 _returnvalue_2)) (* (- (`KismetMathLibrary.FClamp` _returnvalue_4 (`self.min_off`) (`self.max_off`)) _returnvalue_4) _returnvalue_2)) false false :!label _label_2)
      (`PrimitiveComponent.AddForce` (`self.MovableStaticMesh`) (1.0 0.0 0.0) "None" false))))

(event `self.GrabComponent.OnGrabbed`
  (set `self.deifVec` (- (`SceneComponent.K2_GetComponentLocation` (`self.MovableStaticMesh`)) (`SceneComponent.K2_GetComponentLocation` (`/Game/VRTemplate/Blueprints/GrabComponent.MotionControllerRef` (`self.GrabComponent`)))))
  (goto _label :!via `Open`))

(event `self.GrabComponent.OnDropped`
  (`|ExecutionSequence`
    (:`then_0`
      (goto _label :!via `Close`))
    (:`then_1`
      (`SceneComponent.K2_SetWorldLocation` (`self.HandAnchor`) (`SceneComponent.K2_GetComponentLocation` (`self.MovableStaticMesh`)) false false)
      (goto _label_2))))

(fn `UserConstructionScript`)