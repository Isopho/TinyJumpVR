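; Physics-driven VR movable with a primary and a secondary mesh, each grabbed by motion controller and slid along its own arrow axis.
; BeginPlay sets up linear constraint limits from the offset settings and enables collision after a short delay.
; While grabbed, Tick projects hand movement onto the axis and applies distance-scaled force, cut near the target so damping settles it.
; Speed drives movement audio volume; relative impact velocity scales throttled hit sounds.
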(event `self.ReceiveBeginPlay`
  (bind _output_get (set `self.Primary_Mesh_Start_Transform` (`SceneComponent.K2_GetComponentToWorld` (`self.PrimaryStaticMesh`))))
  ;[1 1 1] Adjust PhysicsConstraint to enforce the Min_Offset and Max_Offset
  (`SceneComponent.K2_SetWorldLocation` (`self.PrimaryAnchor`) (+ (.location _output_get) (* (`KismetMathLibrary.Normal` (`SceneComponent.GetForwardVector` (`self.PrimaryArrow`))) (/ (+ (`self.Max_Offset`) (`self.Min_Offset`)) 2.0))) false false)
  (`SceneComponent.K2_SetWorldLocation` (`self.PrimaryPhysicsConstraint`) (+ (.location _output_get) (* (`KismetMathLibrary.Normal` (`SceneComponent.GetForwardVector` (`self.PrimaryArrow`))) (/ (+ (`self.Max_Offset`) (`self.Min_Offset`)) 2.0))) false false)
  (`PhysicsConstraintComponent.SetLinearXLimit` (`self.PrimaryPhysicsConstraint`) "LCM_Limited" (`KismetMathLibrary.Abs` (/ (- (`self.Max_Offset`) (`self.Min_Offset`)) 2.0)))
  (`PhysicsConstraintComponent.SetLinearZLimit` (`self.SecondaryPhysicsConstraint`) "LCM_Limited" (`self.Secundary_Max_Offset`))
  (`KismetSystemLibrary.Delay` 0.2)
  (`PrimitiveComponent.SetCollisionResponseToChannel` (`self.PrimaryStaticMesh`) "ECC_GameTraceChannel2" "ECR_Block")
  (`PrimitiveComponent.SetCollisionResponseToChannel` (`self.PrimaryStaticMesh2`) "ECC_GameTraceChannel2" "ECR_Block")
  (`PrimitiveComponent.SetCollisionResponseToChannel` (`self.SecondaryStaticMesh`) "ECC_GameTraceChannel2" "ECR_Block"))

(event `self.ReceiveTick`
  (params (DeltaSeconds :type "Float (single-precision)"))
  (bind _returnvalue (+ (.location (`self.Primary_Mesh_Start_Transform`)) (* (`KismetMathLibrary.Normal` (`KismetMathLibrary.GetForwardVector` (`SceneComponent.K2_GetComponentRotation` (`self.PrimaryArrow`)))) (`self.New_Offset`))))
  (bind _returnvalue_2 (+ (`self.Secondary_Mesh_Grab_Start_Location_0`) (`KismetMathLibrary.ProjectVectorOnToVector` (- (`SceneComponent.K2_GetComponentLocation` (`/Game/VRTemplate/Blueprints/GrabComponent.MotionControllerRef` (`self.SecondaryGrabComponent`))) (`self.Secondary_Hand_Grab_Start_Location_0`)) (`SceneComponent.GetForwardVector` (`self.SecondaryArrow`)))))
  (bind _returnvalue_3 (- (.location (`self.Primary_Mesh_Start_Transform`)) (+ (`self.Primary_Mesh_Grab_Start_Location`) (`KismetMathLibrary.ProjectVectorOnToVector` (- (`SceneComponent.K2_GetComponentLocation` (`/Game/VRTemplate/Blueprints/GrabComponent.MotionControllerRef` (`self.PrimaryGrabComponent`))) (`self.Primary_Hand_Grab_Start_Location`)) (`SceneComponent.GetForwardVector` (`self.PrimaryArrow`))))))
  (bind _returnvalue_4 (`KismetMathLibrary.FClamp` (/ (`KismetMathLibrary.VSize` (- (`SceneComponent.K2_GetComponentLocation` (`self.SecondaryStaticMesh`)) _returnvalue_2)) (`self.Max_Force_Distance`))))
  (bind _returnvalue_5 (`KismetMathLibrary.FClamp` (/ (`KismetMathLibrary.VSize` (- (`SceneComponent.K2_GetComponentLocation` (`self.PrimaryStaticMesh`)) _returnvalue)) (`self.Max_Force_Distance`))))
  (`|ExecutionSequence`
    (:`then_0`
      (`/Engine/EditorBlueprintResources/StandardMacros.Gate` true :!label _label
        (:`Exit`
          (`|ExecutionSequence`
            (:`then_0`
              ;[1 1 1] Disableing when close to target allows the Dampening to take over for a smooth transition
              (if (> _returnvalue_4 0.1)
                (`PrimitiveComponent.AddForce` (`self.SecondaryStaticMesh`) (* (`KismetMathLibrary.GetDirectionUnitVector` (`SceneComponent.K2_GetComponentLocation` (`self.SecondaryStaticMesh`)) _returnvalue_2) (`KismetMathLibrary.Lerp` 0.0 (`self.Drawing_Force`) _returnvalue_4)) "None" false)))
            (:`then_1`
              (bind _returnvalue_6 (`PrimitiveComponent.GetPhysicsLinearVelocity` (`self.SecondaryStaticMesh`) "None"))
              (`AudioComponent.AdjustVolume` (`self.SecondaryMovementAudio`) 0.2 (* (`KismetMathLibrary.FClamp` (/ (`KismetMathLibrary.VSize` _returnvalue_6) 100.0)) (`self.Base Audio Multiplyer`)) "Linear"))))))
    (:`then_1`
      (`/Engine/EditorBlueprintResources/StandardMacros.Gate` true :!label _label_2
        (:`Exit`
          (`|ExecutionSequence`
            (:`then_0`
              (set `self.New_Offset` (`KismetMathLibrary.FClamp` (* (`KismetMathLibrary.VSize` _returnvalue_3) (`KismetMathLibrary.SelectFloat` 1.0 -1.0 (< (`KismetMathLibrary.Dot_VectorVector` _returnvalue_3 (`SceneComponent.GetForwardVector` (`self.PrimaryArrow`))) 0.0))) (`self.Min_Offset`) (`self.Max_Offset`)))
              ;[1 1 1] Disableing when close to target allows the Dampening to take over for a smooth transition
              (if (> _returnvalue_5 0.1)
                (`PrimitiveComponent.AddForce` (`self.PrimaryStaticMesh`) (* (`KismetMathLibrary.GetDirectionUnitVector` (`SceneComponent.K2_GetComponentLocation` (`self.PrimaryStaticMesh`)) _returnvalue) (`KismetMathLibrary.Lerp` 0.0 (`self.Drawing_Force`) _returnvalue_5)) "None" false)))
            (:`then_1`
              (bind _returnvalue_7 (`PrimitiveComponent.GetPhysicsLinearVelocity` (`self.PrimaryStaticMesh`) "None"))
              (`AudioComponent.AdjustVolume` (`self.PrimaryMovementAudio`) 0.2 (* (`KismetMathLibrary.FClamp` (/ (`KismetMathLibrary.VSize` _returnvalue_7) 100.0)) (`self.Base Audio Multiplyer`)) "Linear"))))))))

(event `self.PrimaryGrabComponent.OnGrabbed`
  (`self.Init_Tracking`)
  (`ActorComponent.Activate` (`self.PrimaryMovementAudio`) false)
  (goto _label_2 :!via `Open`))

(event `self.PrimaryGrabComponent.OnDropped`
  (`AudioComponent.AdjustVolume` (`self.PrimaryMovementAudio`) 0.2 0.0 "Linear")
  (goto _label_2 :!via `Close`))

(event `self.SecondaryGrabComponent.OnGrabbed`
  (set `self.Secondary_Mesh_Grab_Start_Location_0` (`SceneComponent.K2_GetComponentLocation` (`self.SecondaryStaticMesh`)))
  (set `self.Secondary_Hand_Grab_Start_Location_0` (`SceneComponent.K2_GetComponentLocation` (`/Game/VRTemplate/Blueprints/GrabComponent.MotionControllerRef` (`self.SecondaryGrabComponent`))))
  (`ActorComponent.Activate` (`self.SecondaryMovementAudio`) false)
  (goto _label :!via `Open`))

(event `self.SecondaryGrabComponent.OnDropped`
  (`AudioComponent.AdjustVolume` (`self.SecondaryMovementAudio`) 0.2 0.0 "Linear")
  (goto _label :!via `Close`))

(event `self.PrimaryStaticMesh.OnComponentHit`
  (params (HitComponent :type "PrimitiveComponent Object Reference") (OtherActor :type "Actor Object Reference") (OtherComp :type "PrimitiveComponent Object Reference") (NormalImpulse :type "Vector Structure") (Hit :type "HitResult Structure (by ref)"))
  (bind _hit_sound (`self.Hit Sound`))
  (set `self.Hit_Location` Hit_ImpactPoint)
  (`self.Calc_Hit_Volume` Hit_Normal (`self.PrimaryStaticMesh`) OtherComp)
  (if (> (`self.Hit_Volume Multiplier`) 0.1) :!label _label_3
    (`/Engine/EditorBlueprintResources/StandardMacros.DoOnce` false :!label _label_4
      (:`Completed`
        (`GameplayStatics.PlaySoundAtLocation` _hit_sound (`self.Hit_Location`) (struct) (`self.Hit_Volume Multiplier`) 1.0 0.0 "/Game/Audio/_Mix/ATT_Emitter_SHRT.ATT_Emitter_SHRT" null null)
        (`KismetSystemLibrary.Delay` (* (`SoundBase.Duration` _hit_sound) 0.8))
        (goto _label_4 :!via `Reset`)))))

(event `self.SecondaryStaticMesh.OnComponentHit`
  (params (HitComponent :type "PrimitiveComponent Object Reference") (OtherActor :type "Actor Object Reference") (OtherComp :type "PrimitiveComponent Object Reference") (NormalImpulse :type "Vector Structure") (Hit :type "HitResult Structure (by ref)"))
  (set `self.Hit_Location` Hit_ImpactPoint)
  (`self.Calc_Hit_Volume` Hit_Normal (`self.SecondaryStaticMesh`) OtherComp)
  (goto _label_3))

(fn `Calc_Hit_Volume`
  (params (Target :type "Vector Structure") (this :type "PrimitiveComponent Object Reference") (other :type "PrimitiveComponent Object Reference"))
  (bind _returnvalue (`PrimitiveComponent.GetPhysicsLinearVelocity` this "None"))
  (bind _returnvalue_2 (`PrimitiveComponent.GetPhysicsLinearVelocity` other "None"))
  (set `self.Hit_Volume Multiplier` (* (`KismetMathLibrary.FClamp` (/ (`KismetMathLibrary.VSize` (`KismetMathLibrary.ProjectVectorOnToVector` (- _returnvalue _returnvalue_2) Target)) 50.0)) (`self.Base Audio Multiplyer`))))

(fn `Init_Tracking`
  (set `self.Primary_Mesh_Grab_Start_Location` (`SceneComponent.K2_GetComponentLocation` (`self.PrimaryStaticMesh`)))
  (set `self.Primary_Hand_Grab_Start_Location` (`SceneComponent.K2_GetComponentLocation` (`/Game/VRTemplate/Blueprints/GrabComponent.MotionControllerRef` (`self.PrimaryGrabComponent`)))))

(fn `UserConstructionScript`)