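; Test grabbable small cube Blueprint that is pulled toward the motion controller holding it.
; GrabComponent's grab and drop events toggle a Grabbed flag.
; While grabbed, Tick applies a force to the static mesh along the normalized direction to the controller, scaled by DrawingForce, so the pull does not vary with distance.
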(event `self.ReceiveBeginPlay`
  (set `self.grabbed` false))

(event `self.ReceiveTick`
  (params (DeltaSeconds :type "Float (single-precision)"))
  (if (`self.grabbed`)
    (`PrimitiveComponent.AddForce` (`self.StaticMesh`) (* (`KismetMathLibrary.Normal` (- (`SceneComponent.K2_GetComponentLocation` (`/Game/VRTemplate/Blueprints/GrabComponent.MotionControllerRef` (`self.GrabComponent`))) (`SceneComponent.K2_GetComponentLocation` (`self.StaticMesh`)))) (`self.DrawingForce`)) "None" false)))

(event `self.GrabComponent.OnGrabbed`
  (set `self.grabbed` true))

(event `self.GrabComponent.OnDropped`
  (set `self.grabbed` false))

(fn `UserConstructionScript`)