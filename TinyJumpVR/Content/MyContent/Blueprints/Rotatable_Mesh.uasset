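; Rotatable_Mesh is a VR-grabbable actor whose StaticMesh is pulled by physics force to follow the motion controller rather than being attached to it.
; GrabComponent's grab event stores the hand-to-mesh offset and sets Grabbed; dropping clears it.
; While grabbed, Tick applies AddForce toward the controller, preserving that offset, with DrawingForce scaled linearly by displacement and capped at MaxForceDistance.
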(event `self.ReceiveBeginPlay`
  (set `self.grabbed` false))

(event `self.ReceiveTick`
  (params (DeltaSeconds :type "Float (single-precision)"))
  (bind _returnvalue (- (- (`SceneComponent.K2_GetComponentLocation` (`/Game/VRTemplate/Blueprints/GrabComponent.MotionControllerRef` (`self.GrabComponent`))) (`SceneComponent.K2_GetComponentLocation` (`self.StaticMesh`))) (`self.Hand_Gran_Start_Relative`)))
  (bind _returnvalue_2 (/ (`KismetMathLibrary.VSize` _returnvalue) (`self.Max_Force_Distance`)))
  (if (`self.grabbed`)
    (`PrimitiveComponent.AddForce` (`self.StaticMesh`) (* (`KismetMathLibrary.Normal` _returnvalue) (`self.Drawing_Force`) (`KismetMathLibrary.SelectFloat` 1.0 _returnvalue_2 (> _returnvalue_2 1.0))) "None" false)))

(event `self.GrabComponent.OnGrabbed`
  (set `self.grabbed` true)
  (set `self.Hand_Gran_Start_Relative` (- (`SceneComponent.K2_GetComponentLocation` (`/Game/VRTemplate/Blueprints/GrabComponent.MotionControllerRef` (`self.GrabComponent`))) (`SceneComponent.K2_GetComponentLocation` (`self.StaticMesh`)))))

(event `self.GrabComponent.OnDropped`
  (set `self.grabbed` false))

(fn `UserConstructionScript`)