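; Test Blueprint that detects components tagged VR_Interactable on actors overlapping its sphere.
; Overlap events maintain a set of these components, opening or closing a Tick gate, and attach a Niagara hand effect using each component's mesh on entry.
; While open, Tick selects the last component within sphere radius of the static mesh, not strictly the closest, then draws a debug arrow and samples its distance into a float history.
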(event `self.ReceiveTick`
  (params (DeltaSeconds :type "Float (single-precision)"))
  (bind _closest_vr_interactable (`self.Closest_VR_Interactable`))
  (bind _returnvalue (`SceneComponent.K2_GetComponentLocation` (`self.StaticMesh`)))
  (bind _returnvalue_2 (`SceneComponent.K2_GetComponentLocation` _closest_vr_interactable))
  (`/Engine/EditorBlueprintResources/StandardMacros.Gate` true :!label _label
    (:`Exit`
      (set `self.Closest_VR_Interactable` null)
      (bind _result (`BlueprintSetLibrary.Set_ToArray` (`self.Overlapping_VR_Interactables`)))
      (if (not (`KismetArrayLibrary.Array_IsEmpty` _result))
        (set `self.Closest_VR_Interactable_Distance` (`SphereComponent.GetScaledSphereRadius` (`self.Sphere`)))
        (for _array_element _result
          (if (< (`KismetMathLibrary.Abs` (`KismetMathLibrary.VSize` (- (`SceneComponent.K2_GetComponentLocation` _array_element) (`SceneComponent.K2_GetComponentLocation` (`self.StaticMesh`))))) (`self.Closest_VR_Interactable_Distance`))
            (set `self.Closest_VR_Interactable` _array_element)))
        (if (`KismetSystemLibrary.IsValid` _closest_vr_interactable)
          (bind _output_get (set `self.Closest_VR_Interactable_Distance` (`KismetMathLibrary.Abs` (`KismetMathLibrary.VSize` (- _returnvalue_2 _returnvalue)))))
          (`KismetSystemLibrary.DrawDebugArrow` _returnvalue _returnvalue_2 1.0 (struct :`R` 1.0 :`B` 0.158835 :`A` 1.0) 0.1 1.0)
          (`KismetSystemLibrary.AddFloatHistorySample` _output_get (`self.NewVar_0`)))))))

(event `self.Sphere.OnComponentBeginOverlap`
  (params (OverlappedComponent :type "PrimitiveComponent Object Reference") (OtherActor :type "Actor Object Reference") (OtherComp :type "PrimitiveComponent Object Reference") (OtherBodyIndex :type Integer) (bFromSweep :type Boolean) (SweepResult :type "HitResult Structure (by ref)"))
  (for _array_element (`SceneComponent.GetChildrenComponents` (`Actor.RootComponent` OtherActor) true)
    (if (`ActorComponent.ComponentHasTag` _array_element "VR_Interactable")
      (`BlueprintSetLibrary.Set_Add` (`self.Overlapping_VR_Interactables`) _array_element)
      (`|ExecutionSequence`
        (:`then_0`
          (goto _label :!via `Open`))
        (:`then_1`
          (bind (_returnvalue_location _returnvalue_rotation) (`KismetMathLibrary.BreakTransform` (`SceneComponent.K2_GetComponentToWorld` _array_element)))
          (bind _returnvalue (`NiagaraFunctionLibrary.SpawnSystemAttached` "/Game/MyContent/FX/NES_Hand_Niagara_LS.NES_Hand_Niagara_LS" _array_element "None" _returnvalue_location _returnvalue_rotation "KeepRelativeOffset"))
          (bind _asstatic_mesh_component (cast `StaticMeshComponent` _array_element))
          (`NiagaraFunctionLibrary.OverrideSystemUserVariableStaticMeshComponent` _returnvalue "User.SpawnMesh" _asstatic_mesh_component))))))

(event `self.Sphere.OnComponentEndOverlap`
  (params (OverlappedComponent :type "PrimitiveComponent Object Reference") (OtherActor :type "Actor Object Reference") (OtherComp :type "PrimitiveComponent Object Reference") (OtherBodyIndex :type Integer))
  (bind _overlapping_vr_interactables (`self.Overlapping_VR_Interactables`))
  (for _array_element (`SceneComponent.GetChildrenComponents` (`Actor.RootComponent` OtherActor) true)
    (if (`ActorComponent.ComponentHasTag` _array_element "VR_Interactable")
      (`BlueprintSetLibrary.Set_Remove` _overlapping_vr_interactables _array_element)
      (if (`BlueprintSetLibrary.Set_IsEmpty` _overlapping_vr_interactables)
        (goto _label :!via `Close`)))))

(fn `UserConstructionScript`)