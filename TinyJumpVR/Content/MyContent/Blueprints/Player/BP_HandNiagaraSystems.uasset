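; Player hand particle effect that drives two Niagara systems to react to the closest grabable object.
; On BeginPlay it feeds a skeletal mesh to the NiagaraWS system, sets the base color on both systems and binds to a grabable update event.
; Within detection range, both systems' colors blend with eased distance and NiagaraWS particles are attracted to the object.
; Otherwise attraction turns slightly negative.
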(event `self.ReceiveBeginPlay`
  (`NiagaraFunctionLibrary.OverrideSystemUserVariableSkeletalMeshComponent` (`self.NiagaraWS`) "User.SkeletalMesh" (`self.SkeletalMeshComponent`))
  (`FXSystemComponent.SetColorParameter` (`self.NiagaraLS`) "User.ParticleColor" (`KismetMathLibrary.Conv_ColorToLinearColor` (`self.ParticleColor1`)))
  (`FXSystemComponent.SetColorParameter` (`self.NiagaraWS`) "User.ParticleColor" (`KismetMathLibrary.Conv_ColorToLinearColor` (`self.ParticleColor1`)))
  (add `self.UpdateNiagaraSystem` (delegate `UpdateNiagaraSystem_Event`)))

(event `UpdateNiagaraSystem_Event` :!signature `self.UpdateNiagaraSystem`
  (params (Grabable :type "SceneComponent Object Reference"))
  (bind _output_get (set `self.Closest_Grabable` Grabable))
  (if (`KismetSystemLibrary.IsValid` _output_get)
    (bind _output_get_2 (set `self.Closest_Grabable_Distance` (`KismetMathLibrary.Abs` (`KismetMathLibrary.VSize` (- (`SceneComponent.K2_GetComponentLocation` (`self.DefaultSceneRoot`)) (`SceneComponent.K2_GetComponentLocation` (`self.Closest_Grabable`)))))))
    (if (<= _output_get_2 (`self.DetectionRange`))
      (`FXSystemComponent.SetColorParameter` (`self.NiagaraWS`) "User.ParticleColor" (`KismetMathLibrary.LinearColorLerp` (`KismetMathLibrary.Conv_ColorToLinearColor` (`self.ParicalColor2`)) (`KismetMathLibrary.Conv_ColorToLinearColor` (`self.ParticleColor1`)) (`|EaseFunction` "EaseInOut" (`KismetMathLibrary.FClamp` (/ (`self.Closest_Grabable_Distance`) (`self.DetectionRange`))) 0.0 1.0)))
      (`FXSystemComponent.SetColorParameter` (`self.NiagaraLS`) "User.ParticleColor" (`KismetMathLibrary.LinearColorLerp` (`KismetMathLibrary.Conv_ColorToLinearColor` (`self.ParicalColor2`)) (`KismetMathLibrary.Conv_ColorToLinearColor` (`self.ParticleColor1`)) (`|EaseFunction` "EaseInOut" (`KismetMathLibrary.FClamp` (/ (`self.Closest_Grabable_Distance`) (`self.DetectionRange`))) 0.0 1.0)))
      (`FXSystemComponent.SetVectorParameter` (`self.NiagaraWS`) "User.AttractionPoint" (`SceneComponent.K2_GetComponentLocation` (`self.Closest_Grabable`)))
      (`FXSystemComponent.SetFloatParameter` (`self.NiagaraWS`) "User.AttractionStrength" 2.0)
      (else
        (`FXSystemComponent.SetFloatParameter` (`self.NiagaraWS`) "User.AttractionStrength" -0.1 :!label _label)))
    (else
      (goto _label))))

(fn `UserConstructionScript`)