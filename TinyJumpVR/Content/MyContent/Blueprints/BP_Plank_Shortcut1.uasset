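; BP_Plank_Shortcut1 is a plank that falls under physics to open a shortcut when a linked trigger volume is overlapped.
; On BeginPlay it binds the open event to every volume in its trigger array and keeps the mesh's physics off.
; The first overlap by any actor enables physics and nudges the mesh with a swept offset.
; A short delay then switches physics off again.
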(event `self.ReceiveBeginPlay`
  ;[1 1 1] Initial setup (register trigger volume & disable physics)
  (for _array_element (`self.OpenShortcut_TriggerVolume`)
    (add `self.OnActorBeginOverlap` _array_element (delegate `Event OpenShortcut`)))
  (`PrimitiveComponent.SetSimulatePhysics` (`self.StaticMeshComponent`) false))

(event `Event OpenShortcut` :!signature `self.OnActorBeginOverlap`
  (params (OverlappedActor :type "Actor Object Reference") (OtherActor :type "Actor Object Reference"))
  ;[1 1 1] Start shortcut opening sequence
  (`/Engine/EditorBlueprintResources/StandardMacros.DoOnce` false
    (:`Completed`
      (`PrimitiveComponent.SetSimulatePhysics` (`self.StaticMeshComponent`) true)
      ;[1 1 1] Open shortcut with physics/gravity (disable physics afterwards)
      (`SceneComponent.K2_AddWorldOffset` (`self.StaticMeshComponent`) (-4.0 0.0 4.0) true false)
      (`KismetSystemLibrary.Delay` 1.5)
      (`PrimitiveComponent.SetSimulatePhysics` (`self.StaticMeshComponent`) false))))

(event `self.ReceiveTick`
  (params (DeltaSeconds :type "Float (single-precision)")))

(fn `UserConstructionScript`)