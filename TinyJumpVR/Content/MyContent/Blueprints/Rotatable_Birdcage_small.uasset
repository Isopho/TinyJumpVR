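; VR rotatable birdcage: grabbing it with a motion controller turns its mesh about an anchor, with a Birdcage component physics-constrained to that mesh.
; Grab and drop events toggle a Tick gate, with start transforms saved on grab.
; While held, hand vectors projected onto the rotation plane give a signed angle applied to the mesh rotation.
; A tiny force on the cage keeps the constraint from glitching; bounded sliding logic is present but unused.
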(event `self.ReceiveBeginPlay`
  ;[1 1 1] Save initial tramsform for boundry and rotation calculations
  (set `self.Mesh_Start_Transform` (`SceneComponent.K2_GetComponentToWorld` (`self.StaticMesh`)))
  (`PhysicsConstraintComponent.SetConstrainedComponents` (`self.PhysicsConstraint`) (`self.StaticMesh`) "None" (`self.Birdcage`) "None"))

(event `self.ReceiveTick`
  (params (DeltaSeconds :type "Float (single-precision)"))
  (bind _returnvalue (`KismetMathLibrary.Normal` (`self.Rotation_Plane_Normal`)))
  (bind _returnvalue_2 (`SceneComponent.K2_GetComponentLocation` (`self.Anchor`)))
  (bind _returnvalue_3 (`KismetMathLibrary.Normal` (`KismetMathLibrary.ProjectVectorOnToPlane` (- _returnvalue_2 (`self.Hand_Grab_Start_Location`)) _returnvalue)))
  (bind _returnvalue_4 (`KismetMathLibrary.Normal` (`KismetMathLibrary.ProjectVectorOnToPlane` (- _returnvalue_2 (`SceneComponent.K2_GetComponentLocation` (`/Game/VRTemplate/Blueprints/GrabComponent.MotionControllerRef` (`self.GrabComponent`)))) _returnvalue)))
  (bind _returnvalue_5 (* (`KismetMathLibrary.DegAcos` (`KismetMathLibrary.Dot_VectorVector` _returnvalue_4 _returnvalue_3)) (`KismetMathLibrary.SelectFloat` 1.0 -1.0 (< (`KismetMathLibrary.Dot_VectorVector` (`KismetMathLibrary.Cross_VectorVector` _returnvalue_4 _returnvalue_3) _returnvalue) 0.0))))
  (`/Engine/EditorBlueprintResources/StandardMacros.Gate` true :!label _label
    (:`Exit`
      (`SceneComponent.K2_SetWorldRotation` (`self.StaticMesh`) (`KismetMathLibrary.ComposeRotators` (.rotation (`self.Mesh_Grab_Start_Transform`)) (`KismetMathLibrary.MakeRotator` (* (.x _returnvalue) _returnvalue_5) (* (.y _returnvalue) _returnvalue_5) (* (.z _returnvalue) _returnvalue_5))) false false)
      ;[1 1 1] needed so that the physicsContraint does not bug out
      (`PrimitiveComponent.AddForce` (`self.Birdcage`) (1.0 0.0 0.0) "None" false)
      (set `self.cnt` (+ (`self.cnt`) 1))
      (if (> (`self.cnt`) 50)
        (set `self.cnt` 0)))))

(event `self.GrabComponent.OnGrabbed`
  (`self.Init_Tracking`)
  (goto _label :!via `Open`))

(event `self.GrabComponent.OnDropped`
  (goto _label :!via `Close`))

(fn `Init_Tracking`
  (set `self.Mesh_Grab_Start_Transform` (`SceneComponent.K2_GetComponentToWorld` (`self.StaticMesh`)))
  (set `self.Hand_Grab_Start_Location` (`SceneComponent.K2_GetComponentLocation` (`/Game/VRTemplate/Blueprints/GrabComponent.MotionControllerRef` (`self.GrabComponent`)))))

(fn `UserConstructionScript`)