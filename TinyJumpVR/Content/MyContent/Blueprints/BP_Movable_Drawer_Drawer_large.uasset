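; Large VR drawer that slides along a single axis while held by a motion controller.
; Grabbing records mesh and hand start positions and opens a Tick gate, which dropping closes.
; While open, hand movement is projected onto the mesh's initial forward vector, converted to a clamped signed offset, and applied along the Arrow's forward direction.
; BeginPlay caches the closed-loop reference transform and, after a short delay, blocks a custom trace channel.
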(event `self.ReceiveBeginPlay`
  (set `self.Mesh_Start_Transform` (`SceneComponent.K2_GetComponentToWorld` (`self.StaticMesh`)))
  (`KismetSystemLibrary.Delay` 0.2)
  (`PrimitiveComponent.SetCollisionResponseToChannel` (`self.StaticMesh`) "ECC_GameTraceChannel2" "ECR_Block"))

(event `self.ReceiveTick`
  (params (DeltaSeconds :type "Float (single-precision)"))
  (bind _returnvalue (- (.location (`self.Mesh_Start_Transform`)) (+ (`self.Mesh_Grab_Start_Location`) (`KismetMathLibrary.ProjectVectorOnToVector` (- (`SceneComponent.K2_GetComponentLocation` (`/Game/VRTemplate/Blueprints/GrabComponent.MotionControllerRef` (`self.GrabComponent`))) (`self.Hand_Grab_Start_Location`)) (`KismetMathLibrary.GetForwardVector` (.rotation (`self.Mesh_Start_Transform`)))))))
  (`/Engine/EditorBlueprintResources/StandardMacros.Gate` true :!label _label
    (:`Exit`
      (set `self.New_Offset` (`KismetMathLibrary.FClamp` (* (`KismetMathLibrary.VSize` _returnvalue) (`KismetMathLibrary.SelectFloat` 1.0 -1.0 (< (`KismetMathLibrary.Dot_VectorVector` _returnvalue (`KismetMathLibrary.GetForwardVector` (.rotation (`self.Mesh_Start_Transform`)))) 0.0))) (`self.Min_Offset`) (`self.Max_Offset`)))
      (`SceneComponent.K2_SetWorldLocation` (`self.StaticMesh`) (+ (.location (`self.Mesh_Start_Transform`)) (* (`KismetMathLibrary.Normal` (`KismetMathLibrary.GetForwardVector` (`SceneComponent.K2_GetComponentRotation` (`self.Arrow`)))) (`self.New_Offset`))) false false))))

(event `self.GrabComponent.OnGrabbed`
  (`self.Init_Tracking`)
  (goto _label :!via `Open`))

(event `self.GrabComponent.OnDropped`
  (goto _label :!via `Close`))

(fn `Init_Tracking`
  (set `self.Mesh_Grab_Start_Location` (`SceneComponent.K2_GetComponentLocation` (`self.StaticMesh`)))
  (set `self.Hand_Grab_Start_Location` (`SceneComponent.K2_GetComponentLocation` (`/Game/VRTemplate/Blueprints/GrabComponent.MotionControllerRef` (`self.GrabComponent`)))))

(fn `UserConstructionScript`)