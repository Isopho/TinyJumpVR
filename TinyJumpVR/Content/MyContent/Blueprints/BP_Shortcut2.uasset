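; A one-time shortcut with a physics plank that tips over when the VR third-person character enters one of its trigger volumes.
; Opening plays a sound, enables physics and opens a Tick gate that applies torque until a two-second delay freezes the plank again.
; Plank impacts, except against excluded actors, play throttled hit sounds with volume scaled by angular velocity.
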(event `self.ReceiveBeginPlay`
  ;[1 1 1] Initial setup (register trigger volume & disable physics)
  (for _array_element (`self.OpenShortcut_TriggerVolume`)
    (add `self.OnActorBeginOverlap` _array_element (delegate `Event OpenShortcut`)))
  (`KismetSystemLibrary.Delay` 0.5)
  (`PrimitiveComponent.SetSimulatePhysics` (`self.PlankMesh`) false))

(event `self.ReceiveTick`
  (params (DeltaSeconds :type "Float (single-precision)"))
  ;[1 1 1] Open shortcut with physics (disable physics afterwards)
  (`/Engine/EditorBlueprintResources/StandardMacros.Gate` true :!label _label
    (:`Exit`
      (`PrimitiveComponent.AddTorqueInDegrees` (`self.PlankMesh`) (0.0 -500.0 0.0) "None" true)
      (`KismetSystemLibrary.Delay` 2.0)
      (`PrimitiveComponent.SetSimulatePhysics` (`self.PlankMesh`) false)
      (goto _label :!via `Close`))))

(event `Event OpenShortcut` :!signature `self.OnActorBeginOverlap`
  (params (OverlappedActor :type "Actor Object Reference") (OtherActor :type "Actor Object Reference"))
  ;[1 1 1] Start shortcut opening sequence
  (cast `/Game/MyContent/Blueprints/Player/VRThirdPersonCharacter` OtherActor)
  (`/Engine/EditorBlueprintResources/StandardMacros.DoOnce` false
    (:`Completed`
      (`GameplayStatics.PlaySoundAtLocation` "/Game/MyContent/Audio/Pick_Up_object_03.Pick_Up_object_03" (`SceneComponent.K2_GetComponentLocation` (`self.PlankMesh`)) (struct) 1.0 1.0 0.0 "/Game/Audio/_Mix/ATT_Emitter_SHRT.ATT_Emitter_SHRT" null null)
      (`PrimitiveComponent.SetSimulatePhysics` (`self.PlankMesh`) true)
      (goto _label :!via `Open`))))

(event `CustomEvent`
  (params (DeltaSeconds :type "Float (double-precision)")))

(event `self.PlankMesh.OnComponentHit`
  (params (HitComponent :type "PrimitiveComponent Object Reference") (OtherActor :type "Actor Object Reference") (OtherComp :type "PrimitiveComponent Object Reference") (NormalImpulse :type "Vector Structure") (Hit :type "HitResult Structure (by ref)"))
  (bind _hit_sound (`self.Hit_Sound`))
  (bind _returnvalue (`KismetMathLibrary.FClamp` (/ (`KismetMathLibrary.VSize` (`PrimitiveComponent.GetPhysicsAngularVelocityInDegrees` (`self.PlankMesh`) "None")) 90.0)))
  (if (and (< (`KismetArrayLibrary.Array_Find` (`self.No_Sound_Actors`) OtherActor) 0) (> _returnvalue 0.2))
    (`/Engine/EditorBlueprintResources/StandardMacros.DoOnce` false :!label _label_2
      (:`Completed`
        (`GameplayStatics.PlaySoundAtLocation` _hit_sound Hit_ImpactPoint (struct) _returnvalue 1.0 0.0 "/Game/Audio/_Mix/ATT_Emitter_SHRT.ATT_Emitter_SHRT" null null)
        (`KismetSystemLibrary.Delay` (* (`SoundBase.Duration` _hit_sound) 0.5))
        (goto _label_2 :!via `Reset`)))))

(fn `UserConstructionScript`)