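; Level-ending actor that fades out and opens the EndLevel map when the VR third-person character enters one of its trigger volumes.
; The first valid overlap plays the FadeOut level sequence while a timeline scales music and SFX sound-class volumes down through sound mix overrides, then loads the map.
; Starting volumes come from the Options save game, with fallback defaults, and SFX receives an extra multiplier.
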(event `self.ReceiveBeginPlay`
  ;[1 1 1] Initial setup (register trigger volumes)
  (for _array_element (`self.TriggerVolumes`)
    (add `self.OnActorBeginOverlap` _array_element (delegate `TiggerVolumeEntered`))))

(event `TiggerVolumeEntered` :!signature `self.OnActorBeginOverlap`
  (params (OverlappedActor :type "Actor Object Reference") (OtherActor :type "Actor Object Reference"))
  ;[1 1 1] EndLevel
  (cast `/Game/MyContent/Blueprints/Player/VRThirdPersonCharacter` OtherActor)
  (`/Engine/EditorBlueprintResources/StandardMacros.DoOnce` false
    (:`Completed`
      (bind (_outactor _returnvalue) (`LevelSequencePlayer.CreateLevelSequencePlayer` (`self.FadeOut`)))
      (`MovieSceneSequencePlayer.Play` _returnvalue)
      (bind (_musicvolumeoutput _sfxvolumeoutput) (`self.LoadOptionsSettings`))
      (set `self.MusicStartVolume` _musicvolumeoutput)
      (set `self.SFXStartVolume` (* _sfxvolumeoutput 10.0))
      (bind (_direction _fadealpha) (`Timeline|FadeTimeline` :!via `PlayFromStart`)
        (:`Update`
          (`GameplayStatics.SetSoundMixClassOverride` "/Game/MyContent/Audio/TinySoundMix.TinySoundMix" "/Game/MyContent/Audio/TinyMusic.TinyMusic" (* _fadealpha (`self.MusicStartVolume`)) 1.0 0.0)
          (`GameplayStatics.SetSoundMixClassOverride` "/Game/MyContent/Audio/TinySoundMix.TinySoundMix" "/Game/MyContent/Audio/TinySFX.TinySFX" (* _fadealpha (`self.SFXStartVolume`)) 1.0 0.0))
        (:`Finished`
          (`GameplayStatics.OpenLevel` "EndLevel"))))))

(fn `LoadOptionsSettings`
  (returns (MusicVolumeOutput :type "Float (double-precision)") (SFXVolumeOutput :type "Float (double-precision)"))
  (bind _returnvalue (`GameplayStatics.DoesSaveGameExist` "Options"))
  (if _returnvalue
    (bind _returnvalue_2 (`GameplayStatics.LoadGameFromSlot` "Options"))
    (bind _assave_options (cast `/Game/MyContent/Blueprints/SaveOptions` _returnvalue_2)
      (:`then`
        (return (`/Game/MyContent/Blueprints/SaveOptions.MusicVolume` _assave_options) (`/Game/MyContent/Blueprints/SaveOptions.SFXVolume` _assave_options)))
      (:`CastFailed`
        (`KismetSystemLibrary.PrintString` "Error Loading Save Options" true true (struct :`R` 1.0 :`A` 1.0)))))
  (return 0.5 0.5))

(fn `UserConstructionScript`)