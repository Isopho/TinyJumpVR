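; VR-grabbable cage actor whose mesh can turn, and optionally move, around an anchor on a selectable axis.
; Grabbing disables physics, records start transforms and opens a Tick gate; dropping restores configured physics and closes it.
; Each tick, the signed hand angle around the anchor, projected onto the rotation plane, rotates and/or repositions the mesh.
; Optional location- or rotation-based checks gate this update against min/max offset degrees from the initial pose.
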(event `self.ReceiveBeginPlay`
  ;[1 1 1] Save initial tramsform for boundry and rotation calculations
  (set `self.Mesh_Start_Transform` (`SceneComponent.K2_GetComponentToWorld` (`self.StaticMesh`)))
  (`PhysicsConstraintComponent.SetConstrainedComponents` (`self.PhysicsConstraint`) null "None" (`self.StaticMesh`) "None")
  (set `self.Rotation_Plane_Normal` (`KismetMathLibrary.GreaterGreater_VectorRotator` (select `/Game/MyContent/Blueprints/Enums/RotationAxis` (`self.Rotation_Axis`) :`NewEnumerator0` (1.0 0.0 0.0) :`NewEnumerator1` (0.0 1.0 0.0) :`NewEnumerator2` (0.0 0.0 1.0) :!type "Vector Structure") (`SceneComponent.K2_GetComponentRotation` (`self.Root`))))
  (set `self.Initial_Orientation` (`SceneComponent.GetForwardVector` (`self.Arrow`)))
  (`KismetSystemLibrary.Delay` 0.2)
  (`PrimitiveComponent.SetCollisionResponseToChannel` (`self.StaticMesh`) "ECC_GameTraceChannel2" "ECR_Block"))

(event `self.ReceiveTick`
  (params (DeltaSeconds :type "Float (single-precision)"))
  (bind _returnvalue (`SceneComponent.K2_GetComponentLocation` (`self.Anchor`)))
  (bind _returnvalue_2 (`KismetMathLibrary.RotatorFromAxisAndAngle` (`KismetMathLibrary.Normal` (`self.Rotation_Plane_Normal`)) (`self.Current_Rotation_Angle`)))
  (`/Engine/EditorBlueprintResources/StandardMacros.Gate` true :!label _label
    (:`Exit`
      (`self.Calc_Current_Rotation_Angle`)
      (switch `/Game/MyContent/Blueprints/Enums/RotationCalculationMethod` (`self.Constraint_Calculation_Method`)
        (:`NewEnumerator2`
          (if (`self.Rotate_Mesh`) :!label _label_2
            (`SceneComponent.K2_SetWorldRotation` (`self.StaticMesh`) (`KismetMathLibrary.ComposeRotators` (.rotation (`self.Mesh_Grab_Start_Transform`)) _returnvalue_2) false false))
          (if (`self.Move_Mesh`)
            (`SceneComponent.K2_SetWorldLocation` (`self.StaticMesh`) (+ _returnvalue (`KismetMathLibrary.GreaterGreater_VectorRotator` (- (.location (`self.Mesh_Grab_Start_Transform`)) _returnvalue) _returnvalue_2)) true false))
          ;[1 1 1] debugging
          (set `self.cnt` (+ (`self.cnt`) 1))
          (if (> (`self.cnt`) 100)
            (set `self.cnt` 0)))
        (:`NewEnumerator0`
          (if (`self.Calc_Constrains_Based_On_Location`)
            (goto _label_2)))
        (:`NewEnumerator1`
          (if (`self.Calc_Constrains_Based_On_Rotation`)
            (goto _label_2)))))))

(event `self.GrabComponent.OnGrabbed`
  (`PrimitiveComponent.SetSimulatePhysics` (`self.StaticMesh`) false)
  (`self.Init_Tracking`)
  (goto _label :!via `Open`))

(event `self.GrabComponent.OnDropped`
  (`PrimitiveComponent.SetSimulatePhysics` (`self.StaticMesh`) (`self.Simulate_Main_Mesh_Physics`))
  (goto _label :!via `Close`))

(fn `Calc_Current_Rotation_Angle`
  (bind _returnvalue (`KismetMathLibrary.Normal` (`self.Rotation_Plane_Normal`)))
  (bind _returnvalue_2 (`SceneComponent.K2_GetComponentLocation` (`self.Anchor`)))
  (bind _returnvalue_3 (`KismetMathLibrary.Normal` (`KismetMathLibrary.ProjectVectorOnToPlane` (- _returnvalue_2 (`self.Hand_Grab_Start_Location`)) _returnvalue)))
  (bind _returnvalue_4 (`KismetMathLibrary.Normal` (`KismetMathLibrary.ProjectVectorOnToPlane` (- _returnvalue_2 (`SceneComponent.K2_GetComponentLocation` (`/Game/VRTemplate/Blueprints/GrabComponent.MotionControllerRef` (`self.GrabComponent`)))) _returnvalue)))
  (set `self.Current_Rotation_Angle` (* (`KismetMathLibrary.DegAcos` (`KismetMathLibrary.Dot_VectorVector` _returnvalue_4 _returnvalue_3)) (`KismetMathLibrary.SelectFloat` 1.0 -1.0 (< (`KismetMathLibrary.Dot_VectorVector` (`KismetMathLibrary.Cross_VectorVector` _returnvalue_4 _returnvalue_3) (`KismetMathLibrary.Normal` (`self.Rotation_Plane_Normal`))) 0.0)))))

(fn `Init_Tracking`
  (set `self.Mesh_Grab_Start_Transform` (`SceneComponent.K2_GetComponentToWorld` (`self.StaticMesh`)))
  (set `self.Hand_Grab_Start_Location` (`SceneComponent.K2_GetComponentLocation` (`/Game/VRTemplate/Blueprints/GrabComponent.MotionControllerRef` (`self.GrabComponent`))))
  (set `self.Grab_Start_Orientation` (`SceneComponent.GetForwardVector` (`self.Arrow`))))

(fn `UserConstructionScript`)