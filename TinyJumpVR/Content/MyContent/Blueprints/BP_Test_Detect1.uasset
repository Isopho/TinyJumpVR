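; Test actor that detects components tagged VR_Interactable in a sphere and shows the closest one through Niagara effects.
; Overlap events maintain a component-to-distance map, which Tick refreshes to pick the nearest to the static mesh.
; Proximity eases both particle systems' color, and Niagara1 attracts toward the target; an empty map zeroes attraction only on Niagara.
; Debug arrows mark overlaps and the target; child-component search and physics wobble are disconnected.
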(event `self.ReceiveBeginPlay`
  (`FXSystemComponent.SetColorParameter` (`self.Niagara`) "User.ParticleColor" (`KismetMathLibrary.Conv_ColorToLinearColor` (`self.ParticleColor`)))
  (`FXSystemComponent.SetColorParameter` (`self.Niagara1`) "User.ParticleColor" (`KismetMathLibrary.Conv_ColorToLinearColor` (`self.ParticleColor`))))

(event `self.ReceiveTick`
  (params (DeltaSeconds :type "Float (single-precision)"))
  (bind _niagara1 (`self.Niagara1`))
  (bind _closest_vr_interactable (`self.Closest_VR_Interactable`))
  (bind _returnvalue (`SceneComponent.K2_GetComponentLocation` _closest_vr_interactable))
  (bind _returnvalue_2 (`KismetMathLibrary.LinearColorLerp` (`KismetMathLibrary.Conv_ColorToLinearColor` (`self.ParicalColor2`)) (`KismetMathLibrary.Conv_ColorToLinearColor` (`self.ParticleColor`)) (`|EaseFunction` "EaseInOut" (`KismetMathLibrary.FClamp` (/ (`self.Closest_VR_Interactable_Distance`) (`SphereComponent.GetUnscaledSphereRadius` (`self.Sphere`)))) 0.0 1.0)))
  (if (not (`BlueprintMapLibrary.Map_IsEmpty` (`self.Overlapping_VR_Interactables`)))
    (bind _keys (`BlueprintMapLibrary.Map_Keys` (`self.Overlapping_VR_Interactables`)))
    (for _array_element _keys
      (`BlueprintMapLibrary.Map_Add` (`self.Overlapping_VR_Interactables`) _array_element (`KismetMathLibrary.Abs` (`KismetMathLibrary.VSize` (- (`SceneComponent.K2_GetComponentLocation` _array_element) (`SceneComponent.K2_GetComponentLocation` (`self.StaticMesh`)))))))
    (set `self.Closest_VR_Interactable_Distance` (`SphereComponent.GetUnscaledSphereRadius` (`self.Sphere`)))
    (bind _keys_2 (`BlueprintMapLibrary.Map_Keys` (`self.Overlapping_VR_Interactables`)))
    (for _array_element_2 _keys_2
      (bind _value (`BlueprintMapLibrary.Map_Find` (`self.Overlapping_VR_Interactables`) _array_element_2))
      (if (< _value (`self.Closest_VR_Interactable_Distance`))
        (set `self.Closest_VR_Interactable` _array_element_2)
        (set `self.Closest_VR_Interactable_Distance` _value)))
    (if (`KismetSystemLibrary.IsValid` _closest_vr_interactable)
      (`KismetSystemLibrary.DrawDebugArrow` (`SceneComponent.K2_GetComponentLocation` (`self.StaticMesh`)) _returnvalue 1.0 (struct :`R` 1.0 :`B` 0.929991 :`A` 1.0) 0.1 0.5)
      (`FXSystemComponent.SetColorParameter` (`self.Niagara1`) "User.ParticleColor" _returnvalue_2)
      (`FXSystemComponent.SetColorParameter` (`self.Niagara`) "User.ParticleColor" _returnvalue_2)
      (`FXSystemComponent.SetVectorParameter` _niagara1 "User.AttractionPoint" _returnvalue)
      (`FXSystemComponent.SetFloatParameter` _niagara1 "User.AttractionStrength" 1.0)
      (else
        (`FXSystemComponent.SetFloatParameter` _niagara1 "User.AttractionStrength" 0.0)))
    (else
      (`FXSystemComponent.SetFloatParameter` (`self.Niagara`) "User.AttractionStrength" 0.0))))

(event `self.Sphere.OnComponentBeginOverlap`
  (params (OverlappedComponent :type "PrimitiveComponent Object Reference") (OtherActor :type "Actor Object Reference") (OtherComp :type "PrimitiveComponent Object Reference") (OtherBodyIndex :type Integer) (bFromSweep :type Boolean) (SweepResult :type "HitResult Structure (by ref)"))
  (`KismetArrayLibrary.Array_Clear` (`self.TempArray`))
  (`KismetArrayLibrary.Array_Add` (`self.TempArray`) OtherComp)
  (for _array_element (`self.TempArray`)
    (if (`ActorComponent.ComponentHasTag` _array_element "VR_Interactable")
      (`BlueprintMapLibrary.Map_Add` (`self.Overlapping_VR_Interactables`) _array_element -1.0)
      (`KismetSystemLibrary.DrawDebugArrow` (`SceneComponent.K2_GetComponentLocation` (`self.StaticMesh`)) (`SceneComponent.K2_GetComponentLocation` _array_element) 1.0 (struct :`G` 1.0 :`B` 0.10955 :`A` 1.0) 1.5 0.5))))

(event `self.Sphere.OnComponentEndOverlap`
  (params (OverlappedComponent :type "PrimitiveComponent Object Reference") (OtherActor :type "Actor Object Reference") (OtherComp :type "PrimitiveComponent Object Reference") (OtherBodyIndex :type Integer))
  (`KismetArrayLibrary.Array_Clear` (`self.TempArray`))
  (`KismetArrayLibrary.Array_Add` (`self.TempArray`) OtherComp)
  (for _array_element (`self.TempArray`)
    (if (`ActorComponent.ComponentHasTag` _array_element "VR_Interactable")
      (`BlueprintMapLibrary.Map_Remove` (`self.Overlapping_VR_Interactables`) _array_element)
      (`KismetSystemLibrary.DrawDebugArrow` (`SceneComponent.K2_GetComponentLocation` (`self.StaticMesh`)) (`SceneComponent.K2_GetComponentLocation` _array_element) 1.0 (struct :`R` 1.0 :`G` 0.018845 :`A` 1.0) 1.0 0.5))))

(fn `UserConstructionScript`)